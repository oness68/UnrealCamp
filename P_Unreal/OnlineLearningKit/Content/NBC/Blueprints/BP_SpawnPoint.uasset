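; BP_SpawnPoint is a spawner actor that periodically drops random hurdles into the level while its OnTrigger flag is set.
; Tick accumulates delta time and, roughly every one and a half seconds, builds a transform with random rotation and a random X offset around the actor.
; SpawnHurdle then spawns one of three hurdle Blueprint classes, picked at random and assigned at BeginPlay.
; Nothing in this Blueprint sets OnTrigger.
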(event EventBeginPlay
  (Variables|Default|SetHurdle_1 "/Game/NBC/Blueprints/BP_Hurdle_1.BP_Hurdle_1_C")
  (Variables|Default|SetHurdle_2 "/Game/NBC/Blueprints/BP_Hurdle_2.BP_Hurdle_2_C")
  (Variables|Default|SetHurdle_3 "/Game/NBC/Blueprints/BP_Hurdle_3.BP_Hurdle_3_C"))

(event Collision|EventActorBeginOverlap
  (params (OtherActor :type Actor%20Object%20Reference)))

(event EventTick
  (params (DeltaSeconds :type Float%20%28single-precision%29))
  (bind _returnvalue (Transformation|GetActorTransform))
  (if (Variables|Default|GetOnTrigger)
    (bind _output_get (Variables|Default|SetSpawnTime (+ (Variables|Default|GetSpawnTime) (Utilities|Time|GetWorldDeltaSeconds))))
    (if (> _output_get 1.5)
      (Variables|Default|SetRandTransform (Math|Transform|MakeTransform (Math|Vector|MakeVector (+ (.x (.location _returnvalue)) (Math|Random|RandomFloatinRange -1.35e+03 1.35e+03)) (.y (.location _returnvalue)) (.z (.location _returnvalue))) (Math|Random|RandomRotator false) "1.000000,1.000000,1.000000"))
      (CallFunction|SpawnHurdle)
      (Variables|Default|SetSpawnTime 0.0))))

(fn ConstructionScript)

(fn SpawnHurdle
  (switch int (Math|Random|RandomInteger 3)
    (:0
      (Game|SpawnActorfromClass (Variables|Default|GetHurdle_1) (Variables|Default|GetRandTransform) "Undefined" "MultiplyWithRoot" 0 0))
    (:1
      (Game|SpawnActorfromClass (Variables|Default|GetHurdle_2) (Variables|Default|GetRandTransform) "Undefined" "MultiplyWithRoot" 0 0))
    (:2
      (Game|SpawnActorfromClass (Variables|Default|GetHurdle_3) (Variables|Default|GetRandTransform) "Undefined" "MultiplyWithRoot" 0 0))))
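; Enemy actor that, once its Ontrigger flag is set externally, swells and then moves each frame.
; Tick scales it up by a fixed percentage until a size cap, then applies a local Y offset along with its current scale as a delta transform, independent of delta time.
; Its capsule sets Trigger on any overlapped BP_RunFloor tagged "Run".
; BeginPlay stores the point light's transform in Attack, unused here.
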(event OnComponentBeginOverlap(Capsule)
  (params (OverlappedComponent :type Primitive%20Component%20Object%20Reference) (OtherActor :type Actor%20Object%20Reference) (OtherComp :type Primitive%20Component%20Object%20Reference) (OtherBodyIndex :type Integer) (bFromSweep :type Boolean) (SweepResult :type Hit%20Result%20Structure%20%28by%20ref%29))
  (if (Actor|ActorHasTag OtherActor "Run")
    (bind _asbp_run_floor (Utilities|Casting|CastToBP_RunFloor OtherActor))
    (Variables|/Game/NBC/Blueprints/BP_RunFloor.BP_RunFloor_C|SetTrigger _asbp_run_floor true)))

(event EventBeginPlay
  (Variables|Default|SetOntrigger false)
  (Variables|Default|SetAttack (Transformation|GetWorldTransform (Variables|Default|GetPointLight))))

(event Collision|EventActorBeginOverlap
  (params (OtherActor :type Actor%20Object%20Reference)))

(event EventTick
  (params (DeltaSeconds :type Float%20%28single-precision%29))
  (if (Variables|Default|GetOntrigger)
    (if (< (.x (Transformation|GetActorScale3D)) 65.0)
      (Transformation|SetActorScale3D (* (Transformation|GetActorScale3D) "1.01,1.01,1.01"))
      (else
        (Class|SceneComponent|AddLocalTransform (Variables|Default|GetDefaultSceneRoot) (Math|Transform|MakeTransform "0.000000,5.000000,0.000000" "0, 0, 0" (Transformation|GetActorScale3D)) false false)))))

(fn ConstructionScript)
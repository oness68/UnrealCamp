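; BP_NBCCharacter is a player character with Enhanced Input movement, look and jump, knocked back by hurdles.
; BeginPlay adds the default mapping context, and movement follows control rotation yaw.
; Hitting an actor tagged "Hurdle" applies a fixed world-space velocity impulse and sets a Hit flag that blocks repeat knockbacks.
; Tick clears that flag through a one-second Delay, acting as a cooldown.
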(event Input|EnhancedActionEvents|EnhancedInputActionIA_NBC_Move
  (params (ActionValue :type Vector%202D%20Structure) (ElapsedSeconds :type Float%20%28double-precision%29) (TriggeredSeconds :type Float%20%28double-precision%29) (InputAction :type Input%20Action%20Object%20Reference :default "/Game/NBC/Inputs/IA_NBC_Move.IA_NBC_Move"))
  (Pawn|Input|AddMovementInput (Math|Vector|GetForwardVector (Math|Rotator|MakeRotator 0.0 0.0 (.yaw (Pawn|GetControlRotation (Game|GetPlayerController 0) :!class /Script/Engine.Controller)))) (.x ActionValue) false)
  (Pawn|Input|AddMovementInput (Math|Vector|GetRightVector (Math|Rotator|MakeRotator 0.0 0.0 (.yaw (Pawn|GetControlRotation :!class /Script/Engine.Pawn)))) (.y ActionValue) false))

(event Input|EnhancedActionEvents|EnhancedInputActionIA_NBC_Look
  (params (ActionValue :type Vector%202D%20Structure) (ElapsedSeconds :type Float%20%28double-precision%29) (TriggeredSeconds :type Float%20%28double-precision%29) (InputAction :type Input%20Action%20Object%20Reference :default "/Game/NBC/Inputs/IA_NBC_Look.IA_NBC_Look"))
  ;[1 1 1] Look
  (Pawn|Input|AddControllerYawInput (.x ActionValue))
  (Pawn|Input|AddControllerPitchInput (.y ActionValue)))

(event Input|EnhancedActionEvents|EnhancedInputActionIA_NBC_Jump
  (params (ActionValue :type Boolean) (ElapsedSeconds :type Float%20%28double-precision%29) (TriggeredSeconds :type Float%20%28double-precision%29) (InputAction :type Input%20Action%20Object%20Reference :default "/Game/NBC/Inputs/IA_NBC_Jump.IA_NBC_Jump"))
  (:Started
    (Character|Jump)))

(event EventBeginPlay
  ;[1 1 1] Key Mapping
  (Input|AddMappingContext (PlayerController|LocalPlayerSubsystems|GetEnhancedInputLocalPlayerSubsystem (Game|GetPlayerController 0)) "/Game/NBC/Inputs/IMC_NBC_MappingDefault.IMC_NBC_MappingDefault" 0 "(bIgnoreAllPressedKeysUntilRelease=True,bForceImmediately=False,bNotifyUserSettings=False)"))

(event Collision|EventHit
  (params (MyComp :type Primitive%20Component%20Object%20Reference) (Other :type Actor%20Object%20Reference) (OtherComp :type Primitive%20Component%20Object%20Reference) (bSelfMoved :type Boolean) (HitLocation :type Vector :default "0, 0, 0") (HitNormal :type Vector :default "0, 0, 0") (NormalImpulse :type Vector :default "0, 0, 0") (Hit :type Hit%20Result%20Structure%20%28by%20ref%29))
  (if (Actor|ActorHasTag Other "Hurdle")
    (if (not (Variables|Default|Gethit))
      (Physics|AddImpulse (Variables|Character|GetCharacterMovement) "0.000000,-2000.000000,1000.000000" true)
      (Variables|Default|Sethit true))))

(event EventTick
  (params (DeltaSeconds :type Float%20%28single-precision%29))
  (if (Variables|Default|Gethit)
    (Utilities|FlowControl|Delay 1.0)
    (Variables|Default|Sethit false)))

(fn ConstructionScript)
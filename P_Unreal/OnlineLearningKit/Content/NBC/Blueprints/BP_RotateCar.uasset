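; BP_RotateCar is a car obstacle that circles a pivot and launches the player character on contact.
; On BeginPlay it offsets the SM_PowerCar mesh by Radius along world X, and Tick yaws the actor at Speed, so the car orbits the actor's origin.
; A hit on BP_NBCCharacter launches it with the negated world-space impact point as velocity, so the push depends on map position.
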(event OnComponentHit(SM_PowerCar)
  (params (HitComponent :type Primitive%20Component%20Object%20Reference) (OtherActor :type Actor%20Object%20Reference) (OtherComp :type Primitive%20Component%20Object%20Reference) (NormalImpulse :type Vector :default "0, 0, 0") (Hit :type Hit%20Result%20Structure%20%28by%20ref%29))
  (bind _asbp_nbccharacter (Utilities|Casting|CastToBP_NBCCharacter OtherActor))
  (Character|LaunchCharacter _asbp_nbccharacter (* (.impactpoint Hit) (Math|Conversions|ToVector(Float) -1.0)) false false))

(event EventBeginPlay
  (bind _returnvalue (Transformation|GetActorLocation))
  (Transformation|SetWorldLocation (Variables|Default|GetSM_PowerCar) (Math|Vector|MakeVector (+ (.x _returnvalue) (Variables|Default|GetRadius)) (.y _returnvalue) (.z _returnvalue)) false false))

(event EventTick
  (params (DeltaSeconds :type Float%20%28single-precision%29))
  (Transformation|AddActorLocalRotation (Math|Rotator|MakeRotator 0.0 0.0 (* DeltaSeconds (Variables|Default|GetSpeed))) false false))

(fn ConstructionScript)
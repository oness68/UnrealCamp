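; BP_NPC11 is a rock-paper-scissors NPC, apparently meant to show a random hand above itself when the player is near.
; BeginPlay stores a point derived from its location with a 300-unit Z offset.
; Rand picks a choice, records it in NPC and spawns the matching actor there.
; The player-tag check calling Rand and the timed spawn-and-destroy branch are disconnected, and ActorBeginOverlap is empty, so neither runs.
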(event EventBeginPlay
  (bind _output_get (Variables|Default|Settransfrom (Transformation|GetActorLocation)))
  (Variables|Default|Settransfrom (Math|Transform|TransformLocation (Math|Conversions|ToTransform(Vector) _output_get) "0.000000,0.000000,300.000000")))

(event Collision|EventActorBeginOverlap
  (params (OtherActor :type Actor%20Object%20Reference)))

(fn ConstructionScript)

(fn Rand
  (bind _transfrom (Variables|Default|Gettransfrom))
  (bind _returnvalue (Math|Conversions|ToTransform(Vector) _transfrom))
  (switch int (Math|Random|RandomInteger 3)
    (:0
      (Variables|Default|SetNPC "NewEnumerator0")
      (Game|SpawnActorfromClass "/Game/BP/BP_Rock11.BP_Rock11_C" _returnvalue "Undefined" "MultiplyWithRoot" 0 0))
    (:1
      (Variables|Default|SetNPC "NewEnumerator1")
      (Game|SpawnActorfromClass "/Game/BP/BP_Scissors11.BP_Scissors11_C" _returnvalue "Undefined" "MultiplyWithRoot" 0 0))
    (:2
      (Variables|Default|SetNPC "NewEnumerator3")
      (Game|SpawnActorfromClass "/Game/BP/BP_Paper11.BP_Paper11_C" _returnvalue "Undefined" "MultiplyWithRoot" 0 0))))